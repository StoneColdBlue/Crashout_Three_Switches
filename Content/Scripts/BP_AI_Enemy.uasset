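; BP_AI_Enemy is an AI enemy that turns to face and shoots at the player character when it sees one.
; A PawnSensing sighting of a BP_Character snaps the enemy's rotation toward that character.
; If able to attack, it spawns a bullet at SpawnProjectileLocation and applies damage directly on firing, independent of projectile impact.
; A CanAttack flag with a short Delay limits the fire rate.
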(event `self.PawnSensing.OnSeePawn`
  (params (Pawn :type "Pawn Object Reference"))
  (bind _asbp_character (cast `/Game/Scripts/BP_Character` Pawn))
  (`self.K2_SetActorRotation` (`KismetMathLibrary.FindRelativeLookAtRotation` (`KismetMathLibrary.Conv_VectorToTransform` (`self.K2_GetActorLocation`)) (`self.K2_GetActorLocation` _asbp_character)))
  (if (`self.CanAttack?`)
    (`|SpawnActorFromClass` "/Game/Scripts/Bullets/Bullets.Bullets_C" (`SceneComponent.K2_GetComponentToWorld` (`self.SpawnProjectileLocation`)) "Undefined" "MultiplyWithRoot" null null)
    (`GameplayStatics.ApplyDamage` _asbp_character 3.0)
    (set `self.CanAttack?` false)
    (`KismetSystemLibrary.Delay` 0.5)
    (set `self.CanAttack?` true)))

(fn `UserConstructionScript`)
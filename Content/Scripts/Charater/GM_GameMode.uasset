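; Game mode Blueprint that scatters health and gun ammo pickups across the level when play begins.
; SpawnHealth runs first, then SpawnGuns, each gathering the BP_Spawn_Points actors and looping a fixed number of times to spawn its pickup at a random one.
; Each used point is removed and destroyed so pickups never share one, with no check for running out of points.
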(event `self.ReceiveBeginPlay`
  (`self.SpawnHealth`)
  (`self.SpawnGuns`))

(fn `SpawnGuns`
  (locals (LocalSpawnPoints :type "Array of /Game/Scripts/Pickup/BP_Spawn_Points Object Reference") (LocalItem :type "/Game/Scripts/Pickup/BP_Spawn_Points Object Reference"))
  (bind _outactors (`GameplayStatics.GetAllActorsOfClass` "/Game/Scripts/Pickup/BP_Spawn_Points.BP_Spawn_Points_C"))
  (set `local.LocalSpawnPoints` _outactors)
  (for _ (range 16)
    (set `local.LocalItem` (`KismetArrayLibrary.Array_Random` (`local.LocalSpawnPoints`)))
    (`|SpawnActorFromClass` "/Game/Scripts/Pickup/BP_Gun_Amo_Pick_ups.BP_Gun_Amo_Pick_ups_C" (`KismetMathLibrary.MakeTransform` (`self.K2_GetActorLocation` (`local.LocalItem`))) "AdjustIfPossibleButAlwaysSpawn" "MultiplyWithRoot" null null)
    (`KismetArrayLibrary.Array_RemoveItem` (`local.LocalSpawnPoints`) (`local.LocalItem`))
    (`self.K2_DestroyActor` (`local.LocalItem`))))

(fn `SpawnHealth`
  (locals (LocalSpawnPoints :type "Array of /Game/Scripts/Pickup/BP_Spawn_Points Object Reference") (LocalItem :type "/Game/Scripts/Pickup/BP_Spawn_Points Object Reference"))
  (bind _outactors (`GameplayStatics.GetAllActorsOfClass` "/Game/Scripts/Pickup/BP_Spawn_Points.BP_Spawn_Points_C"))
  (set `local.LocalSpawnPoints` _outactors)
  (for _ (range 10)
    (set `local.LocalItem` (`KismetArrayLibrary.Array_Random` (`local.LocalSpawnPoints`)))
    (`|SpawnActorFromClass` "/Game/Scripts/Pickup/BP_Health_Pick_up.BP_Health_Pick_up_C" (`KismetMathLibrary.MakeTransform` (`self.K2_GetActorLocation` (`local.LocalItem`))) "AdjustIfPossibleButAlwaysSpawn" "MultiplyWithRoot" null null)
    (`KismetArrayLibrary.Array_RemoveItem` (`local.LocalSpawnPoints`) (`local.LocalItem`))
    (`self.K2_DestroyActor` (`local.LocalItem`))))

(fn `UserConstructionScript`)
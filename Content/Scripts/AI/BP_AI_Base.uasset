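; BP_AI_Base is a base AI actor with shooting, roaming, health and respawning.
; Shoot spawns scaled-down AI_Bullets at BulletSpawn, while Roam repeatedly moves to random nearby reachable points after successful moves; neither is triggered here.
; Damage lowers clamped health; at zero it sets IsDead and calls Respawn, which asks GM_GameMode to respawn it and refills health.
; IsDead is never cleared here, so further damage calls Respawn directly.
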(event `self.ReceiveBeginPlay`)

(event `shoot`
  (bind (_returnvalue_location _returnvalue_rotation) (`KismetMathLibrary.BreakTransform` (`SceneComponent.K2_GetComponentToWorld` (`self.Bullet_Spawn`))))
  ;[1 1 1] Gun_Fire
  (`|SpawnActorFromClass` "/Game/Scripts/Bullets/AI_Bullets.AI_Bullets_C" (`KismetMathLibrary.MakeTransform` _returnvalue_location _returnvalue_rotation (0.05 0.05 0.05)) "AlwaysSpawn" "MultiplyWithRoot" null null))

(event `Roam`
  ;[1 1 1] Roam
  (`|AIMoveTo` null (`NavigationSystemV1.K2_GetRandomReachablePointInRadius` (`self.K2_GetActorLocation`) 1000.0 null null) null
    (:`then`
      (`KismetSystemLibrary.Delay` 2.0)
      (`self.Roam`))))

(event `self.ReceiveAnyDamage`
  (params (Damage :type "Float (single-precision)") (DamageType :type "DamageType Object Reference") (InstigatedBy :type "Controller Object Reference") (DamageCauser :type "Actor Object Reference"))
  ;[1 1 1] Heath System
  (if (not (`self.isDead?`))
    (bind _output_get (set `self.Current_Health` (`KismetMathLibrary.FClamp` (- (`self.Current_Health`) Damage) 0.0 (`self.Max_Health`))))
    (if (== _output_get 0.0)
      (set `self.isDead?` true)
      (`self.Respawn`))
    (else
      (`self.Respawn`))))

(event `Respawn`
  ;[1 1 1] respawn
  (bind _asgm_game_mode (cast `/Game/Scripts/Charater/GM_GameMode` (`GameplayStatics.GetGameMode`)))
  (`/Game/Scripts/Charater/GM_GameMode.Respawn AI` _asgm_game_mode self)
  (set `self.Current_Health` (`self.Max_Health`)))

(fn `UserConstructionScript`)